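; BP_Door is a swinging door that opens automatically when the first-person character enters its box trigger and closes when it leaves.
; A timeline drives the door mesh's yaw up to the Angel value, playing on overlap begin and reversing on overlap end.
; Swing side comes from loosely comparing the character's direction to the door's forward vector.
; CanInteract tracks the overlap but does not gate opening.
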(event OnComponentBeginOverlap(BoxTrigger)
  (params (OverlappedComponent :type Primitive%20Component%20Object%20Reference) (OtherActor :type Actor%20Object%20Reference) (OtherComp :type Primitive%20Component%20Object%20Reference) (OtherBodyIndex :type Integer) (bFromSweep :type Boolean) (SweepResult :type Hit%20Result%20Structure%20%28by%20ref%29))
  (bind _asbp_first_person_character_1_cat (Utilities|Casting|CastToBP_FirstPersonCharacter1_CAT OtherActor))
  (Variables|Default|SetCanInteract true)
  (if true
    (Variables|Default|SetDirection (Utilities|Operators|EqualEqual (Math|Vector|Normalize (- (Transformation|GetActorLocation _asbp_first_person_character_1_cat) (Transformation|GetActorLocation))) (Transformation|GetActorForwardVector) 1.0))
    (bind _doortimer (Timeline|DoorTime Play)
      (:Update
        (Transformation|SetRelativeRotation (Variables|Default|GetSM_Door) (Math|Rotator|MakeRotator 0.0 0.0 (* _doortimer (Variables|Default|GetAngel) (Math|Float|SelectFloat 1.0 -1.0 (Variables|Default|GetDirection)))) false false)))))

(event OnComponentEndOverlap(BoxTrigger)
  (params (OverlappedComponent :type Primitive%20Component%20Object%20Reference) (OtherActor :type Actor%20Object%20Reference) (OtherComp :type Primitive%20Component%20Object%20Reference) (OtherBodyIndex :type Integer))
  (Utilities|Casting|CastToBP_FirstPersonCharacter1_CAT OtherActor)
  (Variables|Default|SetCanInteract false)
  (bind _doortimer (Timeline|DoorTime Reverse)
    (:Update
      (Transformation|SetRelativeRotation (Variables|Default|GetSM_Door) (Math|Rotator|MakeRotator 0.0 0.0 (* _doortimer (Variables|Default|GetAngel) (Math|Float|SelectFloat 1.0 -1.0 (Variables|Default|GetDirection)))) false false))))

(fn ConstructionScript)